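; BP_Bat is a bat pawn that chases the player until it is dead.
; The Chase event issues an AI MoveTo toward the player pawn's current X and Y, leaving Z unset.
; On success it waits briefly and moves again if IsDead is false; a failed move ends the loop.
; BeginPlay and Tick are inactive, and nothing in this file calls Chase or sets IsDead.
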(event EventBeginPlay)

(event Collision|EventActorBeginOverlap
  (params (OtherActor :type Actor%20Object%20Reference)))

(event EventTick
  (params (DeltaSeconds :type Float%20%28single-precision%29))
  (|CallParentFunction DeltaSeconds) ; This node is disabled and will not be called.\nDrag off pins to build functionality.
)

(event EventChase
  (bind _returnvalue (Game|Player|GetPlayerPawn 0))
  (bind _returnvalue_2 (Transformation|GetActorLocation _returnvalue))
  (if (not (Variables|Default|GetIsDead?))
    (AI|AIMoveTo self (Math|Vector|MakeVector (.x _returnvalue_2) (.y _returnvalue_2) 0.0) 0 5.0 false :!label _label
      (:OnSuccess
        (if (not (Variables|Default|GetIsDead?))
          (Utilities|FlowControl|Delay 2.0)
          (goto _label))))))

(fn ConstructionScript
  (|CallParentFunction))