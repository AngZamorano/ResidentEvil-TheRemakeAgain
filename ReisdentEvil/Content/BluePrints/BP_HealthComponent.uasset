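; BP_HealthComponent is a health component that tracks damage and depletion for the tank character, enemy dogs and other enemies derived from BP_EnemyBase.
; On BeginPlay it casts its owner to set starting health, overriding the maximum for enemy types, then binds to OnTakeAnyDamage; other owners are never bound.
; Each hit subtracts unclamped damage and broadcasts OnHealthChanged, plus OnHealthDepleted whenever health is at or below zero.
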(event Custom|OnDamageTaken
  (params (DamagedActor :type Actor%20Object%20Reference) (Damage :type Float%20%28single-precision%29) (DamageType :type Damage%20Type%20Object%20Reference) (InstigatedBy :type Controller%20Object%20Reference) (DamageCauser :type Actor%20Object%20Reference))
  (bind _output_get (Variables|Default|SetHealth (- (Variables|Default|GetHealth) Damage)))
  (Default|CallOnHealthChanged _output_get)
  (if (<= (Variables|Default|GetHealth) 0.0)
    (Default|CallOnHealthDepleted)))

(event EventBeginPlay
  (bind _returnvalue (Components|GetOwner))
  (Utilities|Casting|CastToBP_TankCharacter _returnvalue
    (:then
      (Variables|Default|SetHealth (Variables|Default|GetMax%20Health)))
    (:CastFailed
      (Utilities|Casting|CastToBP_EnemyDog _returnvalue
        (:then
          (bind _output_get (Variables|Default|SetMax%20Health 1e+02))
          (Variables|Default|SetHealth _output_get))
        (:CastFailed
          (Utilities|Casting|CastToBP_EnemyBase _returnvalue)
          (bind _output_get_2 (Variables|Default|SetMax%20Health 1.5e+02))
          (Variables|Default|SetHealth _output_get_2)))))
  (EventDispatchers|BindEventtoOnTakeAnyDamage (Components|GetOwner) (delegate Custom|OnDamageTaken)))