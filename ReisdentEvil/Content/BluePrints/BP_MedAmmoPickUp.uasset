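; Medium pistol ammo pickup that the player collects through an Interact event.
; A box trigger shows the tank character's interact prompt on begin overlap and hides it on end overlap.
; Interact casts the player character to BP_TankCharacter, adds a fixed amount of pistol ammo, then destroys the pickup.
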(event OnComponentBeginOverlap(Box)
  (params (OverlappedComponent :type Primitive%20Component%20Object%20Reference) (OtherActor :type Actor%20Object%20Reference) (OtherComp :type Primitive%20Component%20Object%20Reference) (OtherBodyIndex :type Integer) (bFromSweep :type Boolean) (SweepResult :type Hit%20Result%20Structure%20%28by%20ref%29))
  (bind _asbp_tank_character (Utilities|Casting|CastToBP_TankCharacter OtherActor))
  (Widget|SetVisibility (Variables|/Game/BluePrints/BP_TankCharacter.BP_TankCharacter_C|GetInteract%20Ref _asbp_tank_character) "Visible"))

(event OnComponentEndOverlap(Box)
  (params (OverlappedComponent :type Primitive%20Component%20Object%20Reference) (OtherActor :type Actor%20Object%20Reference) (OtherComp :type Primitive%20Component%20Object%20Reference) (OtherBodyIndex :type Integer))
  (bind _asbp_tank_character (Utilities|Casting|CastToBP_TankCharacter OtherActor))
  (Widget|SetVisibility (Variables|/Game/BluePrints/BP_TankCharacter.BP_TankCharacter_C|GetInteract%20Ref _asbp_tank_character) "Hidden"))

(event EventBeginPlay)

(event Collision|EventActorBeginOverlap
  (params (OtherActor :type Actor%20Object%20Reference)))

(event EventTick
  (params (DeltaSeconds :type Float%20%28single-precision%29)))

(event EventInteract
  (bind _asbp_tank_character (Utilities|Casting|CastToBP_TankCharacter (Game|GetPlayerCharacter 0)))
  (Default|AddPistolAmmo _asbp_tank_character 25)
  (Actor|DestroyActor))

(fn ConstructionScript)