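; BP_SingleDoor is a door that swings open or closed on an Interact event.
; Interact checks the Frontbox and Backbox overlaps for a BP_TankCharacter to pick the swing timeline, toggling a shared Opened flag.
; RightSwing and Backrightswing timelines drive the door mesh's relative yaw.
; The back timeline runs inverted, reversing to open and playing from start to close.
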(event EventInteract
  (for _array_element (Collision|GetOverlappingActors (Variables|Default|Getfrontbox) 0 :!class /Script/Engine.PrimitiveComponent)
    (Utilities|Casting|CastToBP_TankCharacter _array_element)
    (if (Variables|Default|Getopened?)
      (Variables|Default|Setopened? false)
      (bind _newtrack_0 (Timeline|RightSwing Reverse)
        (:Update
          (Transformation|SetRelativeRotation (Variables|Default|GetSM_doorHouse_01) (Math|Rotator|MakeRotator 0.0 0.0 _newtrack_0) false false)))
      (else
        (Variables|Default|Setopened? true)
        (Timeline|RightSwing Play))))
  (for _array_element_2 (Collision|GetOverlappingActors (Variables|Default|Getbackbox) 0 :!class /Script/Engine.PrimitiveComponent)
    (Utilities|Casting|CastToBP_TankCharacter _array_element_2)
    (if (Variables|Default|Getopened?)
      (Variables|Default|Setopened? false)
      (Utilities|FlowControl|Sequence
        (:then_1
          (bind _newtrack_0_2 (Timeline|backrightswing PlayFromStart)
            (:Update
              (Transformation|SetRelativeRotation (Variables|Default|GetSM_doorHouse_01) (Math|Rotator|MakeRotator 0.0 0.0 _newtrack_0_2) false false)))))
      (else
        (Variables|Default|Setopened? true)
        (Utilities|FlowControl|Sequence
          (:then_0
            (Timeline|backrightswing Reverse)))))))

(fn ConstructionScript)