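; Pistol Blueprint that the player picks up by interacting, then fires using limited ammo.
; Interact runs once, passing the pistol to BP_TankCharacter's WeaponEquiped, while EquipGun sets the weapon's relative transform.
; Shoot sphere-traces forward from BulletPoint against Pawns, leaving persistent debug shapes, then applies damage and spends a round.
; Reload adds the given amount to current ammo, with no cap.
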(event Custom|Equip%20Gun
  (Transformation|SetRelativeTransform (Variables|Default|GetWeapon) (Math|Transform|MakeTransform "2.500000,12.000000,2.000000" "-17.000000,70.000000,10.000000" "0.750000,0.750000,0.750000") false false))

(event Custom|Reload
  (params (Ammount :type Integer))
  (Variables|Default|SetAmmo (+ Ammount (Variables|Default|GetAmmo))))

(event Custom|shoot
  (bind _bulletpoint (Variables|Default|GetBulletPoint))
  (bind _returnvalue (Transformation|GetWorldLocation _bulletpoint))
  (if (> (Variables|Default|GetAmmo) 0)
    (bind _outhit (Collision|SphereTraceForObjects _returnvalue (+ _returnvalue (* (Math|Vector|GetForwardVector _bulletpoint) 2e+03)) 25.0 (Utilities|Array|MakeArray "ObjectTypeQuery3") false (Utilities|Array|MakeArray self (Variables|Default|GetPlayer%20Ref)) "Persistent"))
    (Game|Damage|ApplyDamage (.hitactor _outhit) 25.0 0 0)
    (Math|Integer|DecrementInt (Variables|Default|GetAmmo))))

(event EventInteract
  (Utilities|FlowControl|DoOnce false
    (:Completed
      (bind _asbp_tank_character (Utilities|Casting|CastToBP_TankCharacter (Game|GetPlayerCharacter 0)))
      (bind _output_get (Variables|Default|SetPlayer%20Ref _asbp_tank_character))
      (Default|WeaponEquiped _output_get self))))

(fn ConstructionScript)