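; BP_ShotGun is a shotgun weapon that the player picks up and fires.
; Interact runs once, adding the gun to BP_TankCharacter's inventory and moving the weapon mesh far away rather than destroying the actor.
; Shoot, while ammo remains, fires several randomly offset sphere traces from BulletPoint against pawns, ignoring itself and the player, damages each hit actor, then spends one ammo.
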(event EventBeginPlay)

(event Collision|EventActorBeginOverlap
  (params (OtherActor :type Actor%20Object%20Reference)))

(event EventTick
  (params (DeltaSeconds :type Float%20%28single-precision%29)))

(event EventShoot
  (bind _bulletpoint (Variables|Default|GetBulletPoint))
  (bind _returnvalue (Transformation|GetWorldLocation _bulletpoint))
  (if (> (Variables|Default|GetAmmo) 0)
    (for _index (range 0 4)
      (bind _outhit (Collision|SphereTraceForObjects _returnvalue (+ _returnvalue (* (Math|Vector|GetForwardVector _bulletpoint) 2e+03) (Math|Random|RandomFloatinRange -1e+02 1e+02) (Math|Random|RandomFloatinRange -1e+02 1e+02) (Math|Random|RandomFloatinRange -1e+02 1e+02)) 25.0 (Utilities|Array|MakeArray "ObjectTypeQuery3") false (Utilities|Array|MakeArray self (Variables|Default|GetPlayer%20Ref)) "ForOneFrame"))
      (Game|Damage|ApplyDamage (.hitactor _outhit) 4e+01 0 0))
    (Math|Integer|DecrementInt (Variables|Default|GetAmmo))))

(event EventInteract
  (Utilities|FlowControl|DoOnce false
    (:Completed
      (bind _asbp_tank_character (Utilities|Casting|CastToBP_TankCharacter (Game|GetPlayerCharacter 0)))
      (bind _output_get (Variables|Default|SetPlayer%20Ref _asbp_tank_character))
      (Default|AddtoInventory _output_get "ShotGun" 1 "/Game/AssetsvilleTown/Meshes/Weapons/SM_Shotgun_01.SM_Shotgun_01" self)
      (Transformation|SetRelativeTransform (Variables|Default|GetWeapon) (Math|Transform|MakeTransform "3000.000000,3000.000000,3000.000000" "0, 0, 0" "1.000000,1.000000,1.000000") false false)
      (Variables|Default|SetPickedUp? true))))

(fn ConstructionScript
  (|CallParentFunction))