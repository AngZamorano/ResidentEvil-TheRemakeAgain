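; Game instance Blueprint that holds the player's inventory and handles enemy save and load.
; Save stores references to up to three BP_EnemyBase actors in a BP_RESave slot, matched by array order.
; Load restores only the first enemy's IsDead, reading the existing SaveFile1 variable rather than the loaded object.
; Three slot checks use BPI_Weapon to swap the cached player's equipped weapon or clear its equipped flag.
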(event Custom|Add%20to%20Inventory
  (params (Item :type String) (Amount :type Integer) (Mesh :type Static%20Mesh%20Object%20Reference) (Actor :type Actor%20Object%20Reference))
  (Utilities|Array|Add (Variables|Default|GetInventory) (Utilities|Struct|MakeBP_StructTest Item Amount Mesh Actor)))

(event Custom|Check%20slot%201
  (bind _inventory (Variables|Default|GetInventory))
  (bind _player_ref (Variables|Default|GetPlayer%20Ref))
  (bind _player_ref_2 (Variables|Default|GetPlayer%20Ref))
  (bind _output (Utilities|Array|Get(acopy) _inventory))
  (bind _weapon_ref (Variables|/Game/BluePrints/BP_TankCharacter.BP_TankCharacter_C|GetWeapon%20Ref _player_ref_2))
  (bind (_item _amount _mesh _blueprint) (Utilities|Struct|BreakBP_StructTest _output))
  (if (not (== _mesh 0))
    (if (Utilities|DoesObjectImplementInterface _blueprint "/Game/BluePrints/BPI_Weapon.BPI_Weapon_C")
      (if (Variables|/Game/BluePrints/BP_TankCharacter.BP_TankCharacter_C|GetHasWeaponEquiped _player_ref_2)
        (if (not (== _weapon_ref _blueprint))
          (Default|Unequiped _weapon_ref)
          (Default|WeaponEquiped _player_ref _blueprint))
        (else
          (Default|WeaponEquiped _player_ref _blueprint)))
      (else
        (Variables|/Game/BluePrints/BP_TankCharacter.BP_TankCharacter_C|SetHasWeaponEquiped _player_ref_2 false)))))

(event Custom|refs
  (bind _asbp_tank_character (Utilities|Casting|CastToBP_TankCharacter (Game|GetPlayerCharacter 0)))
  (Variables|Default|SetPlayer%20Ref _asbp_tank_character))

(event Custom|Check%20slot%202
  (bind _inventory (Variables|Default|GetInventory))
  (bind _player_ref (Variables|Default|GetPlayer%20Ref))
  (bind _player_ref_2 (Variables|Default|GetPlayer%20Ref))
  (bind _output (Utilities|Array|Get(acopy) _inventory 1))
  (bind _weapon_ref (Variables|/Game/BluePrints/BP_TankCharacter.BP_TankCharacter_C|GetWeapon%20Ref _player_ref))
  (bind (_item _amount _mesh _blueprint) (Utilities|Struct|BreakBP_StructTest _output))
  (if (not (== _mesh 0))
    (if (Utilities|DoesObjectImplementInterface _blueprint "/Game/BluePrints/BPI_Weapon.BPI_Weapon_C")
      (if (Variables|/Game/BluePrints/BP_TankCharacter.BP_TankCharacter_C|GetHasWeaponEquiped _player_ref)
        (if (not (== _weapon_ref _blueprint))
          (Default|Unequiped _weapon_ref)
          (Default|WeaponEquiped _player_ref_2 _blueprint))
        (else
          (Default|WeaponEquiped _player_ref_2 _blueprint)))
      (else
        (Variables|/Game/BluePrints/BP_TankCharacter.BP_TankCharacter_C|SetHasWeaponEquiped _player_ref false)))))

(event Custom|Check%20slot%203
  (bind _player_ref (Variables|Default|GetPlayer%20Ref))
  (bind _inventory (Variables|Default|GetInventory))
  (bind _player_ref_2 (Variables|Default|GetPlayer%20Ref))
  (bind _output (Utilities|Array|Get(acopy) _inventory 2))
  (bind _weapon_ref (Variables|/Game/BluePrints/BP_TankCharacter.BP_TankCharacter_C|GetWeapon%20Ref _player_ref_2))
  (bind (_item _amount _mesh _blueprint) (Utilities|Struct|BreakBP_StructTest _output))
  (if (not (== _mesh 0))
    (if (Utilities|DoesObjectImplementInterface _blueprint "/Game/BluePrints/BPI_Weapon.BPI_Weapon_C")
      (if (Variables|/Game/BluePrints/BP_TankCharacter.BP_TankCharacter_C|GetHasWeaponEquiped _player_ref_2)
        (if (not (== _weapon_ref _blueprint))
          (Default|Unequiped _weapon_ref)
          (Default|WeaponEquiped _player_ref _blueprint))
        (else
          (Default|WeaponEquiped _player_ref _blueprint)))
      (else
        (Variables|/Game/BluePrints/BP_TankCharacter.BP_TankCharacter_C|SetHasWeaponEquiped _player_ref_2 false)))))

(event Custom|Save
  (bind _returnvalue (SaveGame|CreateSaveGameObject "/Game/BluePrints/BP_RESave.BP_RESave_C"))
  (Variables|Default|SetSave%20file1 _returnvalue)
  (bind _outactors (Actor|GetAllActorsOfClass "/Game/BluePrints/BP_EnemyBase.BP_EnemyBase_C"))
  (for (_array_element _array_index) _outactors
    (if (== _array_index 0)
      (bind _output_get (Variables|/Game/BluePrints/BP_RESave.BP_RESave_C|Setenemy1 (Variables|Default|GetSave%20file1) _array_element))
      (Development|PrintString (Utilities|GetDisplayName _output_get))
      (elif (== _array_index 1)
        (bind _output_get_2 (Variables|/Game/BluePrints/BP_RESave.BP_RESave_C|Setenemy2 (Variables|Default|GetSave%20file1) _array_element))
        (Development|PrintString (Utilities|GetDisplayName _output_get_2))
        (elif (== _array_index 2)
          (Variables|/Game/BluePrints/BP_RESave.BP_RESave_C|Setenemy3 (Variables|Default|GetSave%20file1) _array_element)))))
  (SaveGame|SaveGametoSlot (Variables|Default|GetSave%20file1) "save file 1"))

(event Custom|Load
  (bind _returnvalue (SaveGame|DoesSaveGameExist "save file 1"))
  (if _returnvalue
    (Development|PrintString "Hello")
    (bind _returnvalue_2 (SaveGame|LoadGamefromSlot "save file 1"))
    (Utilities|Casting|CastToBP_RESave _returnvalue_2)
    (bind _outactors (Actor|GetAllActorsOfClass "/Game/BluePrints/BP_EnemyBase.BP_EnemyBase_C"))
    (for (_array_element _array_index) _outactors
      (if (== _array_index 0)
        (Variables|/Game/BluePrints/BP_EnemyBase.BP_EnemyBase_C|SetIsDead? _array_element (Variables|/Game/BluePrints/BP_EnemyBase.BP_EnemyBase_C|GetIsDead? (Variables|/Game/BluePrints/BP_RESave.BP_RESave_C|Getenemy1 (Variables|Default|GetSave%20file1))))))))