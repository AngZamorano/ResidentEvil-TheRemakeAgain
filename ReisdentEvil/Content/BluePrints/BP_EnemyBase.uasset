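; BP_EnemyBase is an enemy base Blueprint that chases the player once its PawnSensing component sees a pawn.
; While alive, it runs AI MoveTo toward player 0, whichever pawn was seen, and repeats after a short delay only when the move succeeds.
; BP_HealthComponent events print health changes and set IsDead on depletion, which stops new chases and further repeats.
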(event OnSeePawn(PawnSensing)
  (params (Pawn :type Pawn%20Object%20Reference))
  (if (not (Variables|Default|GetIsDead?))
    (AI|AIMoveTo self "0, 0, 0" (Game|Player|GetPlayerPawn 0) 5.0 false :!label _label
      (:OnSuccess
        (if (not (Variables|Default|GetIsDead?))
          (Utilities|FlowControl|Delay 2.0)
          (goto _label))))))

(event OnHealthChanged(BP_HealthComponent)
  (params (NewHealth :type Float%20%28double-precision%29))
  (Development|PrintString (Utilities|String|ToString(Float) NewHealth)))

(event OnHealthDepleted(BP_HealthComponent)
  (Development|PrintString "dead")
  (Variables|Default|SetIsDead? true))

(event EventBeginPlay)

(event Collision|EventActorBeginOverlap
  (params (OtherActor :type Actor%20Object%20Reference)))

(event EventTick
  (params (DeltaSeconds :type Float%20%28single-precision%29)))

(fn ConstructionScript)